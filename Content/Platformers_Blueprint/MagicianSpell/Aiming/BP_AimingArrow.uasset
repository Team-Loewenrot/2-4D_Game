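; Aiming arrow actor for the platformer's magician spell that sits at the player's AimingLine and points along the mouse direction.
; BeginPlay and every Tick run the same update, which flags the player as Spawned and snaps the arrow to AimingLine on a fixed Y plane.
; The deprojected mouse direction, flattened to X/Z and scaled down, becomes the ProjectileMovement velocity, which then sets the arrow's look-at rotation.
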(event EventBeginPlay
  (bind _returnvalue (Game|GetPlayerController 0))
  (bind _returnvalue_2 (Transformation|GetActorLocation))
  (bind (_locationx _locationy) (Game|Player|GetMousePosition _returnvalue))
  (bind _worlddirection (Class|GameplayStatics|DeprojectScreentoWorld _returnvalue (Math|Vector2D|MakeVector2D _locationx _locationy)))
  (bind _asbp_platformers_player (Utilities|Casting|CastToBP_Platformers_Player (Game|GetPlayerCharacter 0)))
  (Variables|/Game/Platformers_Blueprint/BP_Platformers_Player.BP_Platformers_Player_C|SetSpawned _asbp_platformers_player true)
  (bind _output_get (Variables|/Script/Engine.MovementComponent|SetVelocity (Variables|Default|GetProjectileMovement) (Math|Vector|MakeVector (* (.x _worlddirection) 0.1) 0.0 (* (.z _worlddirection) 0.1))))
  (bind _output_get_2 (Variables|Default|SetWorld%20Transform (Transformation|GetWorldTransform (Variables|/Game/Platformers_Blueprint/BP_Platformers_Player.BP_Platformers_Player_C|GetAimingLine _asbp_platformers_player))))
  (Transformation|SetActorTransform (Math|Transform|MakeTransform (Math|Vector|MakeVector (.x (.location _output_get_2)) -1.0001 (.z (.location _output_get_2))) (.rotation _output_get_2) (.scale _output_get_2)))
  (Transformation|SetActorRotation (Math|Rotator|FindLookatRotation _returnvalue_2 (+ _returnvalue_2 _output_get))))

(event Collision|EventActorBeginOverlap
  (params (OtherActor :type Actor%20Object%20Reference)))

(event EventTick
  (params (DeltaSeconds :type Float%20%28single-precision%29))
  (bind _returnvalue (Game|GetPlayerController 0))
  (bind _returnvalue_2 (Transformation|GetActorLocation))
  (bind (_locationx _locationy) (Game|Player|GetMousePosition _returnvalue))
  (bind _worlddirection (Class|GameplayStatics|DeprojectScreentoWorld _returnvalue (Math|Vector2D|MakeVector2D _locationx _locationy)))
  (bind _asbp_platformers_player (Utilities|Casting|CastToBP_Platformers_Player (Game|GetPlayerCharacter 0)))
  (Variables|/Game/Platformers_Blueprint/BP_Platformers_Player.BP_Platformers_Player_C|SetSpawned _asbp_platformers_player true)
  (bind _output_get (Variables|/Script/Engine.MovementComponent|SetVelocity (Variables|Default|GetProjectileMovement) (Math|Vector|MakeVector (* (.x _worlddirection) 0.1) 0.0 (* (.z _worlddirection) 0.1))))
  (bind _output_get_2 (Variables|Default|SetWorld%20Transform (Transformation|GetWorldTransform (Variables|/Game/Platformers_Blueprint/BP_Platformers_Player.BP_Platformers_Player_C|GetAimingLine _asbp_platformers_player))))
  (Transformation|SetActorTransform (Math|Transform|MakeTransform (Math|Vector|MakeVector (.x (.location _output_get_2)) -1.0001 (.z (.location _output_get_2))) (.rotation _output_get_2) (.scale _output_get_2)))
  (Transformation|SetActorRotation (Math|Rotator|FindLookatRotation _returnvalue_2 (+ _returnvalue_2 _output_get))))

(fn ConstructionScript)