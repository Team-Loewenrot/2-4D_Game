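; Magician's second spell, a Paper2D projectile fired toward the mouse cursor in the XZ plane.
; BeginPlay sets velocity from the deprojected cursor direction, and Tick keeps rotation aligned with velocity.
; Overlapping anything but itself or the player applies random damage to all orcs in the overlapped component, stops movement and swaps to an impact flipbook.
; The actor destroys itself after impact or when its non-looping flipbook finishes.
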(event OnComponentBeginOverlap(Sphere)
  (params (OverlappedComponent :type Primitive%20Component%20Object%20Reference) (OtherActor :type Actor%20Object%20Reference) (OtherComp :type Primitive%20Component%20Object%20Reference) (OtherBodyIndex :type Integer) (bFromSweep :type Boolean) (SweepResult :type Hit%20Result%20Structure%20%28by%20ref%29))
  (if (not (or (== OtherActor (Game|GetPlayerCharacter 0)) (== OtherActor self)))
    (Utilities|FlowControl|Sequence
      (:then_0
        (for _array_element (Collision|GetOverlappingActors OverlappedComponent "/Game/Platformers_Enemy/BP_Enemy_Orc.BP_Enemy_Orc_C" :!class /Script/Engine.PrimitiveComponent)
          (Game|Damage|ApplyDamage _array_element (Math|Random|RandomFloatinRange 2e+01 3e+01) 0 self)))
      (:then_1
        (Variables|/Script/Engine.MovementComponent|SetVelocity (Variables|Default|GetProjectileMovement) (Math|Vector|MakeVector 0.0 0.0 0.0))
        (Sprite|SetFlipbook (Variables|Default|GetPaperFlipbook) "/Game/Platformers_Assets/World1/sprites/player/Magician/FireAttack/PlaceholderImpactEffect.PlaceholderImpactEffect")
        (Variables|/Script/Engine.ProjectileMovementComponent|SetProjectileGravityScale (Variables|Default|GetProjectileMovement) 0.0)
        (Variables|Default|SetDestroyed true)
        (Utilities|FlowControl|Delay (Class|PaperFlipbookComponent|GetFlipbookLength (Variables|Default|GetPaperFlipbook)))
        (Actor|DestroyActor)))))

(event OnFinishedPlaying(PaperFlipbook)
  (Actor|DestroyActor))

(event EventBeginPlay
  (bind _returnvalue (Game|GetPlayerController 0))
  (bind _returnvalue_2 (Transformation|GetActorLocation))
  (bind (_locationx _locationy) (Game|Player|GetMousePosition _returnvalue))
  (bind _worlddirection (Class|GameplayStatics|DeprojectScreentoWorld _returnvalue (Math|Vector2D|MakeVector2D _locationx _locationy)))
  (Components|Timeline|SetLooping (Variables|Default|GetPaperFlipbook) false)
  (if (not (Variables|Default|GetDestroyed))
    (bind _output_get (Variables|/Script/Engine.MovementComponent|SetVelocity (Variables|Default|GetProjectileMovement) (Math|Vector|MakeVector (* (.x _worlddirection) 1e+03) 0.0 (* (.z _worlddirection) 1e+03))))
    (Transformation|SetActorRotation (Math|Rotator|FindLookatRotation _returnvalue_2 (+ _returnvalue_2 _output_get)))))

(event Collision|EventActorBeginOverlap
  (params (OtherActor :type Actor%20Object%20Reference)))

(event EventTick
  (params (DeltaSeconds :type Float%20%28single-precision%29))
  (bind _returnvalue (Transformation|GetActorLocation))
  (Transformation|SetActorRotation (Math|Rotator|FindLookatRotation _returnvalue (+ _returnvalue (stale EventBeginPlay _output_get)))))

(fn ConstructionScript)