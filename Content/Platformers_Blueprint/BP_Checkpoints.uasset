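; Checkpoint actor for a platformer that registers itself as the player's current checkpoint when the player character enters its sphere.
; On overlap it finds BP_CheckpointManager and searches CheckpointWithIndexArray for an unbroken entry, identifying itself by exact location match rather than reference.
; It writes that struct back, raising State from 0 to 1, then sets CurrentCheckpointIndex on BP_Platformers_Player.
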(event OnComponentBeginOverlap(Sphere)
  (params (OverlappedComponent :type Primitive%20Component%20Object%20Reference) (OtherActor :type Actor%20Object%20Reference) (OtherComp :type Primitive%20Component%20Object%20Reference) (OtherBodyIndex :type Integer) (bFromSweep :type Boolean) (SweepResult :type Hit%20Result%20Structure%20%28by%20ref%29))
  (if (== OtherActor (Game|GetPlayerCharacter 0))
    (bind _returnvalue (Actor|GetActorOfClass "/Game/Platformers_Blueprint/BP_CheckpointManager.BP_CheckpointManager_C"))
    (bind _array_element (Utilities|Array|ForEachLoopwithBreak (Variables|/Game/Platformers_Blueprint/BP_CheckpointManager.BP_CheckpointManager_C|GetCheckpointWithIndexArray _returnvalue) :!label _label)
      (:LoopBody
        (if (not (.Broken (Utilities|Struct|BreakCheckpointStateStruct _array_element)))
          (if (Utilities|Operators|EqualEqual (Transformation|GetActorLocation (.Checkpoint (Utilities|Struct|BreakCheckpointStateStruct _array_element))) (Transformation|GetActorLocation self) 0.0)
            (if (== (.State (Utilities|Struct|BreakCheckpointStateStruct _array_element)) 0)
              (Utilities|Array|SetArrayElem (Variables|/Game/Platformers_Blueprint/BP_CheckpointManager.BP_CheckpointManager_C|GetCheckpointWithIndexArray _returnvalue) (.Index (Utilities|Struct|BreakCheckpointStateStruct _array_element)) (Utilities|Struct|MakeCheckpointStateStruct (.Checkpoint (Utilities|Struct|BreakCheckpointStateStruct _array_element)) (.Index (Utilities|Struct|BreakCheckpointStateStruct _array_element)) (Class|KismetSystemLibrary|MakeLiteralInteger 1) (.Broken (Utilities|Struct|BreakCheckpointStateStruct _array_element)) (.RespawnPoint (Utilities|Struct|BreakCheckpointStateStruct _array_element))))
              (else
                (Utilities|Array|SetArrayElem (Variables|/Game/Platformers_Blueprint/BP_CheckpointManager.BP_CheckpointManager_C|GetCheckpointWithIndexArray _returnvalue) (.Index (Utilities|Struct|BreakCheckpointStateStruct _array_element)) (Utilities|Struct|MakeCheckpointStateStruct (.Checkpoint (Utilities|Struct|BreakCheckpointStateStruct _array_element)) (.Index (Utilities|Struct|BreakCheckpointStateStruct _array_element)) (.State (Utilities|Struct|BreakCheckpointStateStruct _array_element)) (.Broken (Utilities|Struct|BreakCheckpointStateStruct _array_element)) (.RespawnPoint (Utilities|Struct|BreakCheckpointStateStruct _array_element))))))
            (bind _asbp_platformers_player (Utilities|Casting|CastToBP_Platformers_Player OtherActor))
            (Variables|/Game/Platformers_Blueprint/BP_Platformers_Player.BP_Platformers_Player_C|SetCurrentCheckpointIndex _asbp_platformers_player (.Index (Utilities|Struct|BreakCheckpointStateStruct _array_element)))
            (goto _label Break)))))))

(event EventBeginPlay)

(event Collision|EventActorBeginOverlap
  (params (OtherActor :type Actor%20Object%20Reference)))

(event EventTick
  (params (DeltaSeconds :type Float%20%28single-precision%29)))

(fn ConstructionScript)