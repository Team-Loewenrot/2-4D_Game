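; BP_LayerManager indexes the level's tilemap layers by depth and changes their opacity relative to a given current layer.
; On BeginPlay it gathers tilemap actors tagged IndexedTileMap, bubble-sorts them by ascending Y location (despite the SortTilemapsByZ name) and stores each with its index.
; UpdateTilemapMaterials swaps each tilemap's material, using separate opacity materials for the current layer, lower-index layers and higher-index layers.
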(event Custom|SortTilemapsByZ
  (for _index (range 0 (- (Utilities|Array|Length (Variables|Default|GetTilemapLayers)) 2))
    (for _index_2 (range 0 (Utilities|Operators|Subtract (Utilities|Array|Length (Variables|Default|GetTilemapLayers)) _index 2))
      (if (> (.y (Transformation|GetActorLocation (Utilities|Array|Get(acopy) (Variables|Default|GetTilemapLayers) _index_2))) (.y (Transformation|GetActorLocation (Utilities|Array|Get(acopy) (Variables|Default|GetTilemapLayers) (+ _index_2 1)))))
        (Variables|Default|SetTempTilemap (Utilities|Array|Get(acopy) (Variables|Default|GetTilemapLayers) _index_2))
        (Utilities|Array|SetArrayElem (Variables|Default|GetTilemapLayers) _index_2 (Utilities|Array|Get(acopy) (Variables|Default|GetTilemapLayers) (+ _index_2 1)))
        (Utilities|Array|SetArrayElem (Variables|Default|GetTilemapLayers) (+ _index_2 1) (Variables|Default|GetTempTilemap))))))

(event Custom|AssignIndex
  (bind _outactors (Actor|GetAllActorswithTag "IndexedTileMap"))
  (for _array_element _outactors
    (bind _aspaper_tile_map_actor (Utilities|Casting|CastToPaperTileMapActor _array_element))
    (Utilities|Array|Add (Variables|Default|GetTilemapLayers) _aspaper_tile_map_actor))
  (CallFunction|SortTilemapsbyZ)
  (for (_array_element_2 _array_index) (Variables|Default|GetTilemapLayers)
    (Utilities|Array|Add (Variables|Default|GetTilemapWithIndexArray) (Utilities|Struct|MakeTilemapWithIndexStruct _array_element_2 _array_index))))

(event Custom|UpdateTilemapMaterials
  (params (CurrentLayerIndex :type Integer))
  (bind _array_element (Utilities|Array|ForEachLoopwithBreak (Variables|Default|GetTilemapWithIndexArray))
    (:LoopBody
      (if (== (.LayerIndex (Utilities|Struct|BreakTilemapWithIndexStruct _array_element)) CurrentLayerIndex)
        (Rendering|Material|SetMaterial (Variables|/Script/Paper2D.PaperTileMapActor|GetRenderComponent (.TilemapActor (Utilities|Struct|BreakTilemapWithIndexStruct _array_element))) 0 "/Game/Materials/Opacity1.Opacity1")
        (elif (< (.LayerIndex (Utilities|Struct|BreakTilemapWithIndexStruct _array_element)) CurrentLayerIndex)
          (Rendering|Material|SetMaterial (Variables|/Script/Paper2D.PaperTileMapActor|GetRenderComponent (.TilemapActor (Utilities|Struct|BreakTilemapWithIndexStruct _array_element))) 0 "/Game/Materials/Opacity_Half.Opacity_Half")
          (else
            (Rendering|Material|SetMaterial (Variables|/Script/Paper2D.PaperTileMapActor|GetRenderComponent (.TilemapActor (Utilities|Struct|BreakTilemapWithIndexStruct _array_element))) 0 "/Game/Materials/Opacity_0-1.Opacity_0-1")))))))

(event Collision|EventActorBeginOverlap
  (params (OtherActor :type Actor%20Object%20Reference)))

(event EventTick
  (params (DeltaSeconds :type Float%20%28single-precision%29)))

(event EventBeginPlay
  (CallFunction|AssignIndex))

(fn ConstructionScript)