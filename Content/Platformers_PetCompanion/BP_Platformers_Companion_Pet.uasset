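; Paper2D companion pet for the platformer that follows the player and swaps between idle and walk flipbooks based on velocity.
; It constantly moves forward, while a looping timer flips its facing toward the player's X position.
; Sphere overlaps halt or restore walk speed near the player, and leaving PlayerBounds snaps the pet to the player.
; While the player is phasing, Tick copies the player's Y position onto the pet.
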(event OnComponentBeginOverlap(Sphere)
  (params (OverlappedComponent :type Primitive%20Component%20Object%20Reference) (OtherActor :type Actor%20Object%20Reference) (OtherComp :type Primitive%20Component%20Object%20Reference) (OtherBodyIndex :type Integer) (bFromSweep :type Boolean) (SweepResult :type Hit%20Result%20Structure%20%28by%20ref%29))
  (if (== (== OtherActor (Game|GetPlayerCharacter 0)) (Utilities|Operators|NotEqual(!=) (Transformation|GetActorLocation OtherActor) (Transformation|GetActorLocation) 0.0))
    (Variables|/Script/Engine.CharacterMovementComponent|SetMaxWalkSpeed (Variables|Character|GetCharacterMovement) 0.0)))

(event OnComponentEndOverlap(Sphere)
  (params (OverlappedComponent :type Primitive%20Component%20Object%20Reference) (OtherActor :type Actor%20Object%20Reference) (OtherComp :type Primitive%20Component%20Object%20Reference) (OtherBodyIndex :type Integer))
  (if (== OtherActor (Game|GetPlayerCharacter 0))
    (Variables|/Script/Engine.CharacterMovementComponent|SetMaxWalkSpeed (Variables|Character|GetCharacterMovement) 1.5e+02)))

(event OnComponentEndOverlap(PlayerBounds)
  (params (OverlappedComponent :type Primitive%20Component%20Object%20Reference) (OtherActor :type Actor%20Object%20Reference) (OtherComp :type Primitive%20Component%20Object%20Reference) (OtherBodyIndex :type Integer))
  (bind _returnvalue (Game|GetPlayerCharacter 0))
  (if (== OtherActor _returnvalue)
    (Transformation|SetActorLocation self (Transformation|GetActorLocation _returnvalue) false false)))

(event Custom|MoveForward
  (Pawn|Input|AddMovementInput (Transformation|GetActorForwardVector) 1.0 false))

(event Custom|TargetPlayer
  (Math|Float|CompareFloat (.x (Transformation|GetActorLocation (Game|GetPlayerCharacter 0))) (.x (Transformation|GetActorLocation self))
    (:>
      (Transformation|SetActorRotation "0, 0, 0"))
    (:<
      (Transformation|SetActorRotation "0.000000,180.000000,0.000000"))))

(event Custom|CheckIfPlayerPhasing
  (bind _returnvalue (Transformation|GetActorLocation))
  (bind _asbp_platformers_player (Utilities|Casting|CastToBP_Platformers_Player (Game|GetPlayerCharacter 0)))
  (if (Variables|/Game/Platformers_Blueprint/BP_Platformers_Player.BP_Platformers_Player_C|GetIsPhasing _asbp_platformers_player)
    (Transformation|SetActorLocation (Math|Vector|MakeVector (.x _returnvalue) (.y (Transformation|GetActorLocation _asbp_platformers_player)) (.z _returnvalue)) false false)))

(event Custom|CheckTargetPlayer
  (Utilities|Time|SetTimerbyEvent (delegate Custom|TargetPlayer) 0.1 true))

(event Custom|UpdateAnim
  ;[0.15 0.15 0.15 0.5] UpdateAnimation
  (Sprite|SetFlipbook (Variables|Default|GetSprite) (select (> (Math|Vector|VectorLength (Variables|/Script/Engine.MovementComponent|GetVelocity (Variables|Character|GetCharacterMovement))) 0.0) "/Game/Character/Sprites_Pet/Walk/Root_Walk5.Root_Walk5" "/Game/Character/Sprites_Pet/Idle/Root_Idle3.Root_Idle3")))

(event Collision|EventActorBeginOverlap
  (params (OtherActor :type Actor%20Object%20Reference)))

(event EventTick
  (params (DeltaSeconds :type Float%20%28single-precision%29))
  (CallFunction|MoveForward)
  (CallFunction|UpdateAnim)
  (CallFunction|CheckifPlayerPhasing))

(event EventBeginPlay
  (CallFunction|CheckTargetPlayer))

(fn ConstructionScript)