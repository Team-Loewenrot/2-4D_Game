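; 2D flipbook ghost enemy that constantly moves forward and alternates between homing on the player's X position and wandering.
; A looping timer turns it toward the player; once horizontally aligned, it eases to a halt through a velocity fade timer.
; After its idle/drop-nuke flipbook duration, it resumes speed and stops targeting for several seconds, flipping direction via a DoOnce/FlipFlop cooldown.
; Tick picks the fly or idle flipbook from velocity.
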(event Custom|UpdateAnimation
  (Sprite|SetFlipbook (Variables|Default|GetSprite) (select (> (Math|Vector|VectorLength (Variables|/Script/Engine.MovementComponent|GetVelocity (Variables|Character|GetCharacterMovement))) 0.0) "/Game/Platformers_Enemy/Enemy_Ghost_Sprites/Fly/Enemy_Ghost_Fly.Enemy_Ghost_Fly" "/Game/Platformers_Enemy/Enemy_Ghost_Sprites/Idle/Enemy_Ghost_Idle_OR_DropNuke.Enemy_Ghost_Idle_OR_DropNuke")))

(event Custom|VectorFadeOut
  (bind _charactermovement (Variables|Character|GetCharacterMovement))
  (if (not (Math|Vector|VectorIsNearlyZero (Variables|/Script/Engine.MovementComponent|GetVelocity _charactermovement) 3e+01))
    (Variables|/Script/Engine.MovementComponent|SetVelocity _charactermovement (Math|Interpolation|VInterpTo (Variables|/Script/Engine.MovementComponent|GetVelocity _charactermovement) "0, 0, 0" (Utilities|Time|GetWorldDeltaSeconds) 1.0))
    (else
      (Variables|/Script/Engine.MovementComponent|SetVelocity _charactermovement "0, 0, 0")
      (Utilities|Time|ClearandInvalidateTimerbyHandle (stale Custom|TargetPlayer _returnvalue_7)))))

(event Custom|CheckTargetPlayer
  (bind _returnvalue (Utilities|Time|SetTimerbyEvent (delegate Custom|TargetPlayer) 0.1 true)))

(event Custom|TargetPlayer
  (bind _returnvalue (Game|GetPlayerCharacter 0))
  (bind _self self)
  (bind _charactermovement (Variables|Character|GetCharacterMovement))
  (bind _sprite (Variables|Default|GetSprite))
  (bind _returnvalue_2 (Transformation|GetActorLocation _returnvalue))
  (bind _returnvalue_3 (Transformation|GetActorLocation _self))
  (bind _returnvalue_4 (- (.x _returnvalue_2) 2e+01))
  (bind _returnvalue_5 (+ (.x _returnvalue_2) 2e+01))
  (bind _returnvalue_6 (Math|Float|InRange(Float) (.x _returnvalue_3) _returnvalue_4 _returnvalue_5))
  (if (Variables|Default|GetIsTargetingPlayer)
    (Utilities|FlowControl|Sequence
      (:then_0
        (if (not _returnvalue_6)
          (if (< (.x _returnvalue_2) (.x _returnvalue_3))
            (Transformation|SetActorRotation "0.000000,180.000000,0.000000")
            (else
              (Transformation|SetActorRotation "0, 0, 0")))))
      (:then_1
        (if _returnvalue_6
          (if (not (== (Class|PaperFlipbookComponent|GetFlipbook _sprite) "/Game/Platformers_Enemy/Enemy_Ghost_Sprites/Idle/Enemy_Ghost_Idle_OR_DropNuke.Enemy_Ghost_Idle_OR_DropNuke"))
            (if (!= (Variables|/Script/Engine.CharacterMovementComponent|GetMaxWalkSpeed (Variables|Character|GetCharacterMovement)) 0.0)
              (Variables|/Script/Engine.CharacterMovementComponent|SetMaxWalkSpeed _charactermovement 0.0)
              (bind _returnvalue_7 (Utilities|Time|SetTimerbyEvent (delegate Custom|VectorFadeOut) 0.01 true))
              (if (not (Math|Vector|VectorIsNearlyZero (Variables|/Script/Engine.MovementComponent|GetVelocity _charactermovement) 3e+01))
                (Variables|/Script/Engine.MovementComponent|SetVelocity _charactermovement (Math|Interpolation|VInterpTo (Variables|/Script/Engine.MovementComponent|GetVelocity _charactermovement) "0, 0, 0" (Utilities|Time|GetWorldDeltaSeconds) 1.0))
                (else
                  (Variables|/Script/Engine.MovementComponent|SetVelocity _charactermovement "0, 0, 0")
                  (Utilities|Time|ClearandInvalidateTimerbyHandle _returnvalue_7))))
            (else
              (Utilities|FlowControl|Delay (Class|PaperFlipbookComponent|GetFlipbookLength _sprite))
              (Variables|Default|SetIsTargetingPlayer false)
              (if (!= (Variables|/Script/Engine.CharacterMovementComponent|GetMaxWalkSpeed (Variables|Character|GetCharacterMovement)) 1.2e+02) :!label _label
                (Variables|/Script/Engine.CharacterMovementComponent|SetMaxWalkSpeed (Variables|Character|GetCharacterMovement) 1.2e+02))))
          (else
            (goto _label)))))
    (else
      (Utilities|Time|ClearandInvalidateTimerbyHandle (stale Custom|CheckTargetPlayer _returnvalue))
      (Utilities|FlowControl|Delay 6.0)
      (Variables|Default|SetIsTargetingPlayer true)
      (CallFunction|CheckTargetPlayer))))

(event Custom|WalkRandomly
  (if (not (Variables|Default|GetIsTargetingPlayer))
    (Utilities|FlowControl|DoOnce false
      (:Completed
        (Utilities|FlowControl|FlipFlop
          (:A
            (Transformation|SetActorRotation "0, 0, 0")
            (Utilities|FlowControl|Delay 3.0)
            (CallFunction|ResetWalkRandomlyCooldown))
          (:B
            (Transformation|SetActorRotation "0.000000,180.000000,0.000000")
            (Utilities|FlowControl|Delay 3.0)
            (CallFunction|ResetWalkRandomlyCooldown)))))))

(event Custom|ResetWalkRandomlyCooldown
  (Utilities|FlowControl|DoOnce false) ; enters at Reset
)

(event EventTick
  (params (DeltaSeconds :type Float%20%28single-precision%29))
  (CallFunction|UpdateAnimation)
  (Pawn|Input|AddMovementInput (Transformation|GetActorForwardVector) 1.0 true)
  (CallFunction|WalkRandomly))

(event EventBeginPlay
  (Variables|Default|SetIsTargetingPlayer true)
  (CallFunction|CheckTargetPlayer))

(fn ConstructionScript)